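; Griswold is a sprite-based enemy character that chases the player once pawn sensing spots them and is destroyed when damage depletes its health.
; Each tick it moves toward that target and picks one of four facings from its forward vector in the player's local space, a Doom-style directional-sprite technique.
; Facing changes trigger flipbook selection by velocity, though only front and back views are handled and no attack animation is assigned.
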(event OnSeePawn(PawnSensing1)
  (params (Pawn :type Pawn%20Object%20Reference))
  (bind _returnvalue (Game|Player|GetPlayerPawn 0))
  ;[1 1 1] Sees the player
  (if (== Pawn _returnvalue)
    (Variables|Default|Settarget _returnvalue)))

(event Custom|UpdateAnimation
  (bind _returnvalue (Transformation|GetVelocity))
  (bind _returnvalue_2 (Math|Vector|VectorLength _returnvalue))
  (bind _returnvalue_3 (> _returnvalue_2 0.0))
  (bind _returnvalue_4 (select _returnvalue_3 "NewEnumerator1" "NewEnumerator0"))
  ;[1 1 1] Animation
  (switch Utilities|FlowControl|Switch|SwitchonSpriteFacing (Variables|Default|GetCurrentFacing)
    (:NewEnumerator0
      (Sprite|SetFlipbook (Variables|Default|GetSpriteboard) (Utilities|Select :Index _returnvalue_4 :NewEnumerator0 "/Game/Flipbooks/FGrisStand.FGrisStand" :NewEnumerator1 "/Game/Flipbooks/FGriswalk.FGriswalk" :NewEnumerator2 0)))
    (:NewEnumerator3
      (Sprite|SetFlipbook (Variables|Default|GetSpriteboard) (Utilities|Select :Index _returnvalue_4 :NewEnumerator0 "/Game/Flipbooks/BGrisWalk.BGriswalk" :NewEnumerator1 "/Game/Flipbooks/BGrisWalk.BGriswalk" :NewEnumerator2 0)))))

(event EventTick
  (params (DeltaSeconds :type Float%20%28single-precision%29))
  (bind _target (Variables|Default|Gettarget))
  ;[1 1 1] Tick
  (CallFunction|UpdateFacing)
  (if (Utilities|IsValid _target)
    (AI|Navigation|SimpleMovetoActor (Pawn|GetController) _target)))

(event EventAnyDamage
  (params (Damage :type Float%20%28single-precision%29) (DamageType :type Damage%20Type%20Object%20Reference) (InstigatedBy :type Controller%20Object%20Reference) (DamageCauser :type Actor%20Object%20Reference))
  ;[1 1 1] Damaged
  (Variables|Default|SetHealth (- (Variables|Default|GetHealth) (Math|Float|Floor Damage)))
  (if (<= (Variables|Default|GetHealth) 0)
    (Actor|DestroyActor)))

(fn ConstructionScript)

(fn UpdateFacing
  (bind _returnvalue (Transformation|GetActorForwardVector))
  (bind _returnvalue_2 (Game|Player|GetPlayerPawn 0))
  (bind _returnvalue_3 (Transformation|GetActorTransform _returnvalue_2))
  (bind _returnvalue_4 (- "0, 0, 0" _returnvalue))
  (bind _returnvalue_5 (Math|Transform|InverseTransformDirection _returnvalue_3 _returnvalue_4))
  (bind (_x _y) (Math|Vector|BreakVector _returnvalue_5))
  (bind _returnvalue_6 (Class|KismetMathLibrary|DegAtan2 _y _x))
  (bind _returnvalue_7 (+ _returnvalue_6 3.6e+02))
  (bind _returnvalue_8 (Math|Float|%(Float) _returnvalue_7 3.6e+02))
  (if (or (< _returnvalue_8 45.0) (> _returnvalue_8 315.0))
    (LocalVariables|SetnewFacing "NewEnumerator0")
    (elif (< _returnvalue_8 135.0)
      (LocalVariables|SetnewFacing "NewEnumerator2")
      (elif (< _returnvalue_8 225.0)
        (LocalVariables|SetnewFacing "NewEnumerator3")
        (else
          (LocalVariables|SetnewFacing "NewEnumerator1")))))
  (if (!= (LocalVariables|GetnewFacing) (Variables|Default|GetCurrentFacing))
    (Variables|Default|SetCurrentFacing (LocalVariables|GetnewFacing))
    (CallFunction|UpdateAnimation)))