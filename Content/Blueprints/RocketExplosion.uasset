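; Rocket explosion actor that deals one burst of area damage and then cleans itself up.
; On its first Tick, the server applies damage to every overlapping actor, crediting the instigator's controller, then destroys the collider.
; The actor destroys itself when its Graphics particle system finishes.
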(event OnSystemFinished(Graphics)
  (params (PSystem :type Particle%20System%20Component%20Object%20Reference))
  (Actor|DestroyActor))

(event EventTick
  (params (DeltaSeconds :type Float%20%28single-precision%29))
  (Utilities|FlowControl|DoOnce false
    (:Completed
      (Networking|SwitchHasAuthority
        (:Authority
          (for _array_element (Collision|GetOverlappingActors 0 :!class /Script/Engine.PrimitiveComponent)
            (Game|Damage|ApplyDamage _array_element (Variables|Default|GetDamage) (Game|GetInstigatorController) 0))
          (Components|DestroyComponent (Variables|Default|GetCollider)))))))

(fn ConstructionScript)