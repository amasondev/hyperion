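; CeilingLight is a ceiling light fixture Blueprint that sets up its look and lighting in the construction script.
; LightColor drives the point light and the Color parameter of a dynamic material instance on mesh slot 1.
; Intensity is applied to both the point and spot lights, while the spot light's color is fixed to black rather than following LightColor.
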(fn ConstructionScript
  (bind _intensity (Variables|Default|GetIntensity))
  (bind _lightcolor (Variables|Default|GetlightColor))
  (bind _mesh (Variables|Default|GetMesh))
  ;[1 1 1] Color
  (Rendering|Components|Light|SetLightColor (Variables|Default|GetPointLight1) _lightcolor)
  (Rendering|Components|Light|SetLightColor :self (Variables|Default|GetSpotLight1))
  (bind _returnvalue (Rendering|Material|CreateDynamicMaterialInstance (Rendering|Material|GetMaterial _mesh 1) :!class /Script/Engine.KismetMaterialLibrary))
  (Rendering|Material|SetVectorParameterValue _returnvalue "Color" _lightcolor :!class /Script/Engine.MaterialInstanceDynamic)
  (Rendering|Material|SetMaterial _mesh 1 _returnvalue)
  (Rendering|Components|Light|SetIntensity (Variables|Default|GetPointLight1) _intensity)
  (Rendering|Components|Light|SetIntensity (Variables|Default|GetSpotLight1) _intensity))