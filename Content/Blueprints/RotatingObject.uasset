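; RotatingObject tracks which of four sides (Forward, Left, Backward, Right) it shows relative to the player pawn's orientation.
; Each tick, UpdateFacing transforms its negated forward vector into pawn local space and sorts the yaw angle into 90-degree sectors.
; The test uses only rotations, ignoring where the pawn stands.
; A facing change stores the value and calls UpdateAnim, an empty function here.
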(event EventTick
  (params (DeltaSeconds :type Float%20%28single-precision%29))
  (CallFunction|UpdateFacing))

(fn ConstructionScript)

(fn UpdateFacing
  (bind _returnvalue (Game|Player|GetPlayerPawn 0))
  (bind _returnvalue_2 (Transformation|GetActorForwardVector))
  (bind _returnvalue_3 (Transformation|GetActorTransform _returnvalue))
  (bind _returnvalue_4 (- "0, 0, 0" _returnvalue_2))
  (bind _returnvalue_5 (Math|Transform|InverseTransformDirection _returnvalue_3 _returnvalue_4))
  (bind (_x _y) (Math|Vector|BreakVector _returnvalue_5))
  (bind _returnvalue_6 (Class|KismetMathLibrary|DegAtan2 _y _x))
  (bind _returnvalue_7 (+ _returnvalue_6 3.6e+02))
  (bind _returnvalue_8 (Math|Float|%(Float) _returnvalue_7 3.6e+02))
  (Utilities|IsValid _returnvalue
    (:Is%20Valid
      (if (or (< _returnvalue_8 45.0) (> _returnvalue_8 315.0))
        (LocalVariables|SetnewFacing "Forward")
        (elif (< _returnvalue_8 135.0)
          (LocalVariables|SetnewFacing "Left")
          (elif (< _returnvalue_8 225.0)
            (LocalVariables|SetnewFacing "Backward")
            (else
              (LocalVariables|SetnewFacing "Right")))))
      (if (!= (LocalVariables|GetnewFacing) (Variables|Default|GetCurrentFacing))
        (Variables|Default|SetCurrentFacing (LocalVariables|GetnewFacing))
        (CallFunction|UpdateAnim)))))

(fn UpdateAnim)