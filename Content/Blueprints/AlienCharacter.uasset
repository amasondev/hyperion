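; Alien enemy character that chases and melee-attacks players, drawn as a directional flipbook sprite.
; The server targets the first player it sees or whoever last damaged it, moves toward them and triggers attacks in range.
; Attacks play animation and random sound, with damage and knockback applied on authority.
; Each tick picks one of four facings relative to player 0, mirroring the sprite for Right outside attacks.
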(event OnSeePawn(PawnSensing1)
  (params (Pawn :type Pawn%20Object%20Reference))
  ;[1 1 1] Sees the player (server)
  (Networking|SwitchHasAuthority
    (:Authority
      (Utilities|IsValid (Variables|Default|Gettarget)
        (:Is%20Valid
          _)
        (:Is%20Not%20Valid
          (bind _asfpsplayer (Utilities|Casting|CastToFPSPlayer Pawn))
          (Variables|Default|Settarget _asfpsplayer)))
      (bind _returnvalue (Transformation|GetDistanceTo (Variables|Default|Gettarget)))
      (if (and (<= _returnvalue (Variables|Attributes|GetAttackDistance)) (not (Variables|Runtimestates|GetAttacking)))
        (CallFunction|AttackEvent)))))

(event Custom|AttackEvent
  ;[1 1 1] Client attack
  (CallFunction|Attack (Variables|Default|Gettarget)))

(event EventTick
  (params (DeltaSeconds :type Float%20%28single-precision%29))
  (bind _target (Variables|Default|Gettarget))
  ;[1 1 1] Tick
  (CallFunction|UpdateFacing)
  (Networking|SwitchHasAuthority
    (:Authority
      (if (Utilities|IsValid _target)
        (AI|Navigation|SimpleMovetoActor (Pawn|GetController) _target)))))

(event EventAnyDamage
  (params (Damage :type Float%20%28single-precision%29) (DamageType :type Damage%20Type%20Object%20Reference) (InstigatedBy :type Controller%20Object%20Reference) (DamageCauser :type Actor%20Object%20Reference))
  ;[1 1 1] Damaged
  (Variables|Default|Settarget (Pawn|GetControlledPawn InstigatedBy))
  (Variables|Attributes|SetHealth (- (Variables|Attributes|GetHealth) (Math|Float|Floor Damage)))
  (if (<= (Variables|Attributes|GetHealth) 0)
    (Actor|DestroyActor)))

(fn ConstructionScript
  (Variables|Visuals|SetOriginalScale (Variables|/Script/Engine.SceneComponent|GetRelativeScale3D (Variables|Default|GetSpriteboard))))

(fn UpdateFacing
  (bind _returnvalue (Transformation|GetActorForwardVector))
  (bind _returnvalue_2 (Game|Player|GetPlayerPawn 0))
  (bind _returnvalue_3 (Transformation|GetActorTransform _returnvalue_2))
  (bind _returnvalue_4 (- "0, 0, 0" _returnvalue))
  (bind _returnvalue_5 (Math|Transform|InverseTransformDirection _returnvalue_3 _returnvalue_4))
  (bind (_x _y) (Math|Vector|BreakVector _returnvalue_5))
  (bind _returnvalue_6 (Class|KismetMathLibrary|DegAtan2 _y _x))
  (bind _returnvalue_7 (+ _returnvalue_6 3.6e+02))
  (bind _returnvalue_8 (Math|Float|%(Float) _returnvalue_7 3.6e+02))
  (Utilities|IsValid _returnvalue_2
    (:Is%20Valid
      (if (or (< _returnvalue_8 45.0) (> _returnvalue_8 315.0))
        (LocalVariables|SetnewFacing "Forward")
        (elif (< _returnvalue_8 135.0)
          (LocalVariables|SetnewFacing "Left")
          (elif (< _returnvalue_8 225.0)
            (LocalVariables|SetnewFacing "Backward")
            (else
              (LocalVariables|SetnewFacing "Right")))))
      (if (!= (LocalVariables|GetnewFacing) (Variables|Visuals|GetCurrentFacing))
        (Variables|Visuals|SetCurrentFacing (LocalVariables|GetnewFacing))
        (CallFunction|UpdateAnim)))))

(fn UpdateAnim
  (bind _currentfacing (Variables|Visuals|GetCurrentFacing))
  (bind _animations (Variables|Visuals|GetAnimations))
  (bind _spriteboard (Variables|Default|GetSpriteboard))
  (bind _spriteboard_2 (Variables|Default|GetSpriteboard))
  (bind _originalscale (Variables|Visuals|GetOriginalScale))
  (bind (_x _y _z) (Math|Vector|BreakVector _originalscale))
  (if (Variables|Runtimestates|GetAttacking)
    (bind _returnvalue (Class|AnimationStore|GetFlipbook _animations "Attacking" _currentfacing))
    (Sprite|SetFlipbook _spriteboard _returnvalue)
    (else
      (bind _returnvalue_2 (Class|AnimationStore|GetFlipbook _animations (select (> (Math|Vector|VectorLength (Transformation|GetVelocity)) 0.0) "Running" "Idle") _currentfacing))
      (Sprite|SetFlipbook _spriteboard _returnvalue_2)
      (if (Utilities|Enum|Equal(Enum) (Variables|Visuals|GetCurrentFacing) "Right")
        (Transformation|SetRelativeScale3D _spriteboard_2 (Math|Vector|MakeVector (- 0.0 _x) _y _z))
        (else
          (Transformation|SetRelativeScale3D _spriteboard_2 (Variables|Visuals|GetOriginalScale)))))))

(fn Attack
  (params (Target :type Pawn%20Object%20Reference))
  (LocalVariables|SetlocalTarget Target)
  ;[1 1 1] Animate
  (Variables|Runtimestates|SetAttacking true)
  (bind _returnvalue (Class|AnimationStore|GetFlipbook (Variables|Visuals|GetAnimations) "Attacking" (Variables|Visuals|GetCurrentFacing)))
  (CallFunction|UpdateAnim)
  ;[1 1 1] Play Sound
  (Audio|PlaySoundatLocation (Utilities|Select :Index (Math|Random|RandomIntegerinRange 0 2) :Option%200 "/Game/Sounds/attack1.attack1" :Option%201 "/Game/Sounds/attack2.attack2" :Option%202 "/Game/Sounds/attack3.attack3") (Transformation|GetActorLocation) 1.0 (Math|Random|RandomFloatinRange 0.9 1.1))
  ;[1 1 1] Deal Damage
  (Utilities|IsValid _returnvalue
    (:Is%20Valid
      (Utilities|Time|SetTimerbyFunctionName 0 "StopAttack" (Class|PaperFlipbook|GetTotalDuration _returnvalue))
      (Networking|SwitchHasAuthority
        (:Authority
          (Game|Damage|ApplyDamage (LocalVariables|GetlocalTarget) (Math|Conversions|ToFloat(Integer) (Variables|Attributes|GetDamage)) 0 self)
          ;[1 1 1] Apply Force
          (bind _ascharacter (Utilities|Casting|CastToCharacter (LocalVariables|GetlocalTarget)))
          (Physics|AddImpulse _ascharacter (* (Transformation|GetActorForwardVector) (Variables|Attributes|GetAttackForce)) true))))))

(fn StopAttack
  (Variables|Runtimestates|SetAttacking false))