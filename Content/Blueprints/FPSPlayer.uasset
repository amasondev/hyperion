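; First-person player Blueprint that handles movement and hitscan pistol shooting.
; Horizontal and Vertical axes add movement along the actor's right and forward vectors.
; Fire1 plays a Paper2D flipbook animation and gunshot, then line-traces from the camera on Visibility with debug drawing and applies damage to the hit actor.
; When the fire animation finishes, the weapon flipbook reverts to its default pistol.
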(event OnFinishedPlaying(Weapon)
  ;[1 1 1] Shooting
  (Sprite|SetFlipbook (Variables|Default|GetWeapon) "/Game/Flipbooks/Pistol.Pistol"))

(event Input|ActionEvents|InputActionFire1
  (bind _returnvalue (Game|GetPlayerCameraManager 0))
  (bind _weapon (Variables|Default|GetWeapon))
  (bind _returnvalue_2 (Transformation|GetActorLocation _returnvalue))
  ;[1 1 1] Shooting
  (:Pressed
    (Components|Timeline|SetLooping _weapon false)
    (Sprite|SetFlipbook _weapon "/Game/Flipbooks/Pistol_Fire.Pistol_Fire")
    (Components|Timeline|PlayfromStart _weapon)
    (Class|GameplayStatics|PlaySoundAttached "/Game/Sounds/Gunshot1.Gunshot1" _weapon)
    (bind _outhit (Collision|LineTraceByChannel _returnvalue_2 (+ (* (Transformation|GetActorForwardVector _returnvalue) (Variables|Default|GetWeaponRange)) _returnvalue_2) "TraceTypeQuery1" false 0 "ForDuration"))
    (Game|Damage|ApplyDamage (.HitActor (Collision|BreakHitResult _outhit)) (Math|Conversions|ToFloat(Integer) (Variables|Default|GetWeaponDamage)) 0 0)))

(event Input|AxisEvents|InputAxisHorizontal
  (params (AxisValue :type Float%20%28single-precision%29))
  ;[1 1 1] Movement
  (Pawn|Input|AddMovementInput (Transformation|GetActorRightVector) AxisValue false))

(event Input|AxisEvents|InputAxisVertical
  (params (AxisValue :type Float%20%28single-precision%29))
  ;[1 1 1] Movement
  (Pawn|Input|AddMovementInput (Transformation|GetActorForwardVector) AxisValue false))

(fn ConstructionScript)