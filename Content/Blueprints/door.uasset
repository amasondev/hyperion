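; A sliding double door that opens when a player interacts with it, triggered only on the server.
; A timeline's distance track offsets the Left and Right panels in opposite directions along local Y from locations cached in the construction script.
; Event tracks on the same timeline play the open and close sounds at the door's location, and the timeline rewinds to zero when finished.
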(event Custom|OpenTheDoor
  (bind _returnvalue (Transformation|GetActorLocation))
  ;[1 1 1] Open the door if server
  (bind _distance (Timeline|Timeline_0 Play)
    (:Update
      (Transformation|SetRelativeLocation (Variables|Default|Getleft) (+ (Math|Vector|MakeVector 0.0 _distance 0.0) (Variables|Default|GetleftInitialLocation)) false)
      (Transformation|SetRelativeLocation (Variables|Default|Getright) (- (Variables|Default|GetrightInitialLocation) (Math|Vector|MakeVector 0.0 _distance 0.0)) false))
    (:Finished
      (Components|Timeline|SetPlaybackPosition (Variables|Default|GetTimeline_0) 0.0 false))
    (:Open
      (Audio|PlaySoundatLocation "/Game/Sounds/dsdoropn.dsdoropn" _returnvalue 1.0 1.0 0.0 "/Game/Sounds/Default.Default"))
    (:Close
      (Audio|PlaySoundatLocation "/Game/Sounds/dsdorcls.dsdorcls" _returnvalue 1.0 1.0 0.0 "/Game/Sounds/Default.Default"))))

(event EventPlayerInteracted
  (Networking|SwitchHasAuthority
    (:Authority
      (CallFunction|OpentheDoor))))

(fn ConstructionScript
  (bind _returnvalue (Transformation|GetRelativeTransform))
  (Variables|Default|SetleftInitialLocation (.Location (Math|Transform|BreakTransform _returnvalue)))
  (bind _returnvalue_2 (Transformation|GetRelativeTransform))
  (Variables|Default|SetrightInitialLocation (.Location (Math|Transform|BreakTransform _returnvalue_2))))